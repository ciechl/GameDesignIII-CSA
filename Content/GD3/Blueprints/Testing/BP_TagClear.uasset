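; BP_TagClear is a test actor that switches the role tag of any actor overlapping it between "Cleaner" and "Painter".
; On overlap it overwrites the second tag slot with "Painter" if the actor's tags contain "Cleaner", otherwise with "Cleaner".
; Actors without a second tag get "Cleaner" appended instead.
; Both paths then print every tag for debugging, and a leftover ArraySet node never runs.
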(event `self.ReceiveActorBeginOverlap`
  (params (OtherActor :type "Actor Object Reference"))
  (bind _tags (`Actor.Tags` OtherActor))
  (bind _tags_2 (`Actor.Tags` OtherActor))
  (if (`KismetArrayLibrary.Array_IsValidIndex` (`Actor.Tags` OtherActor) 1)
    (if (`KismetArrayLibrary.Array_Contains` (`Actor.Tags` OtherActor) "Cleaner")
      (`KismetArrayLibrary.Array_Set` (`Actor.Tags` OtherActor) 1 "Painter")
      (else
        (`KismetArrayLibrary.Array_Set` _tags 1 "Cleaner")))
    (for _array_element _tags
      (`KismetSystemLibrary.PrintString` (`KismetStringLibrary.Conv_NameToString` _array_element)))
    (else
      (`KismetArrayLibrary.Array_Add` _tags_2 "Cleaner")
      (for _array_element_2 _tags_2
        (`KismetSystemLibrary.PrintString` (`KismetStringLibrary.Conv_NameToString` _array_element_2))))))

(fn `UserConstructionScript`)