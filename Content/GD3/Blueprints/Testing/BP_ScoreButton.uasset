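; BP_ScoreButton is a test actor that changes the team scores when another actor overlaps it.
; On overlap it casts the game instance to BP_GameManager, passes in its ScoreAmount and TeamScore settings, then calls UpdateScore.
; It prints the resulting Clean and Paint scores to screen, or a debug message if the cast fails.
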(event `self.ReceiveActorBeginOverlap`
  (params (OtherActor :type "Actor Object Reference"))
  (bind _asbp_game_manager (cast `/Game/GD3/Blueprints/BP_GameManager` (`GameplayStatics.GetGameInstance`))
    (:`then`
      (set `/Game/GD3/Blueprints/BP_GameManager.ScoreChange` (`self.ScoreAmount`) _asbp_game_manager)
      (set `/Game/GD3/Blueprints/BP_GameManager.UpdatePaintScore` (`self.TeamScore`) _asbp_game_manager)
      (`/Game/GD3/Blueprints/BP_GameManager.UpdateScore` _asbp_game_manager)
      (`KismetSystemLibrary.PrintString` (`KismetStringLibrary.Concat_StrStr` "Clean Score: " (`KismetStringLibrary.Conv_IntToString` (`/Game/GD3/Blueprints/BP_GameManager.CleanScore` _asbp_game_manager))))
      (`KismetSystemLibrary.PrintString` (`KismetStringLibrary.Concat_StrStr` "Paint Score: " (`KismetStringLibrary.Conv_IntToString` (`/Game/GD3/Blueprints/BP_GameManager.PaintScore` _asbp_game_manager)))))
    (:`CastFailed`
      (`KismetSystemLibrary.PrintString` "Not Doing The Casting Thing"))))

(fn `UserConstructionScript`)