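; Paintable display piece, such as a museum statue or pirate prop, that feeds paint and clean scores to BP_GameManager.
; On BeginPlay a server event scales the mesh by pack and assigns it, falling back to Hebe.
; "Paint" hits increment a counter, scoring only if also tagged "Projectile".
; Other "Projectile" hits destroy the hit component's children (decals), submit the count as a non-team score and reset it.
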(event `self.ReceiveBeginPlay`
  (`self.Server_InitializeObject`))

(event `Server_InitializeObject`
  (`self.InitializeObject`))

(event `self.ReceiveHit`
  (params (MyComp :type "PrimitiveComponent Object Reference") (Other :type "Actor Object Reference") (OtherComp :type "PrimitiveComponent Object Reference") (bSelfMoved :type Boolean) (HitLocation :type "Vector Structure") (HitNormal :type "Vector Structure") (NormalImpulse :type "Vector Structure") (Hit :type "HitResult Structure (by ref)"))
  (bind _children (`SceneComponent.GetChildrenComponents` (`self.SelfRef`) false))
  (`|ExecutionSequence`
    (:`then_0`
      ;[0.3322 0 1] Creates A Reference To Scene Component
      (`/Engine/EditorBlueprintResources/StandardMacros.DoOnce` false
        (:`Completed`
          (set `self.SelfRef` MyComp))))
    (:`then_1`
      (if (`self.ActorHasTag` Other "Paint")
        (`self.DecalPainting` Other)
        (`/Engine/EditorBlueprintResources/StandardMacros.DoOnce` false :!label _label
          (:`Completed`
            (`KismetSystemLibrary.Delay` 0.02)
            (`self.K2_DestroyActor` Other)
            (goto _label :!via `Reset`)))
        (elif (`self.ActorHasTag` Other "Projectile")
          ;[1 1 1] Clears Away Any Decals on This Object
          (for _array_element _children :!label _label_2
            (`ActorComponent.K2_DestroyComponent` _array_element)
            (`KismetSystemLibrary.Delay` 0.2)
            (goto _label_2))
          (`|ExecutionSequence`
            (:`then_0`
              (`KismetArrayLibrary.Array_Clear` _children))
            (:`then_1`
              (`self.ClearDecal`))
            (:`then_2`
              (`/Engine/EditorBlueprintResources/StandardMacros.DoOnce` false :!label _label_3
                (:`Completed`
                  (`KismetSystemLibrary.Delay` 0.02)
                  (`self.K2_DestroyActor` Other)
                  (goto _label_3 :!via `Reset`))))))))))

(fn `CheckIfNullObject`
  (`/Engine/EditorBlueprintResources/StandardMacros.IsValid` (`self.DisplayObject`)
    (:`Is Not Valid`
      (set `self.IsNull` true))))

(fn `ClearDecal`
  (set `self.ScoreAmount` (`self.PointCheck`))
  (set `self.TeamScore` false)
  (`self.UpdateScore`)
  (set `self.PointCheck` 0))

(fn `DecalPainting`
  (params (Bullet :type "Actor Object Reference"))
  (if true
    (`|ExecutionSequence`
      (:`then_0`
        (`/Engine/EditorBlueprintResources/StandardMacros.IncrementInt` (`self.PointCheck`)))
      (:`then_1`
        (if (`self.ActorHasTag` Bullet "Projectile")
          (if (not (== (`self.DefaultScoreAmount`) (`self.ScoreAmount`)))
            (set `self.ScoreAmount` (`self.DefaultScoreAmount`)))
          (set `self.TeamScore` true)
          (`self.UpdateScore`))))))

(fn `InitializeObject`
  (if (`self.PiratePack?`)
    (`self.MuseumPackScale`)
    (else
      (`self.PiratePackScale`)))
  (`self.SetDisplayObject`))

(fn `MuseumPackScale`
  (if (== (`self.DisplayObject`) "/Game/Museum/Meshes/SM_Philosopher.SM_Philosopher")
    (`SceneComponent.SetRelativeScale3D` (`self.ArtPiece`) (1.0 1.0 1.0))
    (elif (== (`self.DisplayObject`) "/Game/Museum/Meshes/SM_Hebe.SM_Hebe")
      (`SceneComponent.SetRelativeScale3D` (`self.ArtPiece`) (2.5 2.5 2.5)))))

(fn `PiratePackScale`
  (if (== (`self.DisplayObject`) "/Game/Ship/Ship/Meshes/SM_Cannon_00.SM_Cannon_00")
    (`SceneComponent.SetRelativeScale3D` (`self.ArtPiece`) (1.0 1.0 1.0))
    (elif (== (`self.DisplayObject`) "/Game/Ship/Lanterns/Meshes/SM_Lantern_12.SM_Lantern_12")
      (`SceneComponent.SetRelativeScale3D` (`self.ArtPiece`) (1.0 1.0 1.0))
      (elif (== (`self.DisplayObject`) "/Game/Ship/Pirate/Meshes/SM_Pirate_Cannon_Ball_00.SM_Pirate_Cannon_Ball_00")
        (`SceneComponent.SetRelativeScale3D` (`self.ArtPiece`) (1.0 1.0 1.0))
        (elif (== (`self.DisplayObject`) "/Game/Ship/Pirate/Meshes/SM_Pirate_Globe_00_Line001.SM_Pirate_Globe_00_Line001")
          (`SceneComponent.SetRelativeScale3D` (`self.ArtPiece`) (1.0 1.0 1.0))
          (elif (== (`self.DisplayObject`) "/Game/Ship/Pirate/Meshes/SM_Pirate_Orb_00_Crystalball.SM_Pirate_Orb_00_Crystalball")
            (`SceneComponent.SetRelativeScale3D` (`self.ArtPiece`) (1.0 1.0 1.0))
            (elif (== (`self.DisplayObject`) "/Game/Ship/Pirate/Meshes/SM_Pirate_Pistol_00_Cube_002.SM_Pirate_Pistol_00_Cube_002")
              (`SceneComponent.SetRelativeScale3D` (`self.ArtPiece`) (1.0 1.0 1.0))
              (elif (== (`self.DisplayObject`) "/Game/Ship/Pirate/Meshes/SM_Pirate_Spyglass_00.SM_Pirate_Spyglass_00")
                (`SceneComponent.SetRelativeScale3D` (`self.ArtPiece`) (1.0 1.0 1.0))
                (elif (== (`self.DisplayObject`) "/Game/Ship/Pirate/Meshes/SM_Pirate_Sword_00.SM_Pirate_Sword_00")
                  (`SceneComponent.SetRelativeScale3D` (`self.ArtPiece`) (1.0 1.0 1.0)))))))))))

(fn `SetDisplayObject`
  (bind _artpiece (`self.ArtPiece`))
  (bind _artpiece_2 (`self.ArtPiece`))
  (bind _displayobject (`self.DisplayObject`))
  (`self.CheckIfNullObject`)
  (if (`self.IsNull`)
    (`StaticMeshComponent.SetStaticMesh` _artpiece_2 "/Game/Museum/Meshes/SM_Hebe.SM_Hebe")
    (`PrimitiveComponent.SetMaterial` _artpiece_2 0 "/Game/StarterContent/LevelPrototyping/Materials/MI_PrototypeGrid_Gray_02.MI_PrototypeGrid_Gray_02")
    (else
      (`StaticMeshComponent.SetStaticMesh` _artpiece _displayobject)
      (`PrimitiveComponent.SetMaterial` _artpiece 0 (`StaticMesh.GetMaterial` _displayobject 0)))))

(fn `UpdateScore`
  (bind _asbp_game_manager (cast `/Game/GD3/Blueprints/BP_GameManager` (`GameplayStatics.GetGameInstance`))
    (:`then`
      (set `/Game/GD3/Blueprints/BP_GameManager.ScoreChange` (`self.ScoreAmount`) _asbp_game_manager)
      (set `/Game/GD3/Blueprints/BP_GameManager.UpdatePaintScore` (`self.TeamScore`) _asbp_game_manager)
      (`/Game/GD3/Blueprints/BP_GameManager.UpdateScore` _asbp_game_manager))
    (:`CastFailed`
      (`KismetSystemLibrary.PrintString` "Not Doing The Casting Thing"))))

(fn `UserConstructionScript`)