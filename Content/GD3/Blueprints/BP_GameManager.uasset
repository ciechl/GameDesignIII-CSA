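; BP_GameManager holds the score of a match between a painting team and a cleaning team.
; UpdateScore acts as a tug-of-war, adding ScoreChange to the team selected by the UpdatePaintScore flag and subtracting it from the other.
; When the gaining team would reach MaxScore, its score is set to that maximum and the opposing score drops to zero.
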(fn `UpdateScore`
  (if (`self.UpdatePaintScore`)
    (if (> (`self.MaxScore`) (+ (`self.PaintScore`) (`self.ScoreChange`)))
      ;[1 1 1] Add Score to Painting Team
      (set `self.PaintScore` (+ (`self.PaintScore`) (`self.ScoreChange`)))
      (set `self.CleanScore` (- (`self.CleanScore`) (`self.ScoreChange`)))
      (else
        (set `self.PaintScore` (`self.MaxScore`))
        (set `self.CleanScore` 0)))
    (elif (> (`self.MaxScore`) (+ (`self.CleanScore`) (`self.ScoreChange`)))
      ;[1 1 1] Add Score to Cleaning Team
      (set `self.CleanScore` (+ (`self.CleanScore`) (`self.ScoreChange`)))
      (set `self.PaintScore` (- (`self.PaintScore`) (`self.ScoreChange`)))
      (else
        (set `self.CleanScore` (`self.MaxScore`))
        (set `self.PaintScore` 0)))))