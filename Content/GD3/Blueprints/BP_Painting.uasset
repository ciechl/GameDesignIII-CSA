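; Framed painting actor that sets up a chosen or random frame and art mesh, with fallbacks, plus a paintable surface.
; BeginPlay creates and clears a render target and gives PaintArea a dynamic material, without binding the target to it here.
; PaintFunction traces from the camera and draws polygons at the hit UV, left mouse painting and right erasing.
; Its only call is in unwired logic, so painting never runs from this graph.
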(event `self.ReceiveBeginPlay`
  (`self.InitializeArt`)
  (bind _returnvalue (`KismetRenderingLibrary.CreateRenderTarget2D` 512 512 "RTF_RGBA8"))
  (bind _output_get (set `self.PaintableCanvas` _returnvalue))
  (`KismetRenderingLibrary.ClearRenderTarget2D` _output_get (`TextureRenderTarget2D.ClearColor` _output_get))
  (bind _returnvalue_2 (`KismetMaterialLibrary.CreateDynamicMaterialInstance` "/Game/GD3/Blueprints/PaintMechanic/BaseMechanic/M_PaintSurfaceBase.M_PaintSurfaceBase"))
  (`PrimitiveComponent.SetMaterial` (`self.PaintArea`) 0 _returnvalue_2))

(event `self.ReceiveTick`
  (params (DeltaSeconds :type "Float (single-precision)")))

(fn `CheckIfNullPainting`
  (`/Engine/EditorBlueprintResources/StandardMacros.IsValid` (`self.Art`)
    (:`Is Valid`
      _)
    (:`Is Not Valid`
      (set `self.Art` "/Game/Assets/Museum/Meshes/SM_PicturePlane.SM_PicturePlane")
      (set `self.ArtNull` true)))
  (`/Engine/EditorBlueprintResources/StandardMacros.IsValid` (`self.PictureFrame`)
    (:`Is Not Valid`
      (set `self.PictureFrame` "/Game/Assets/Museum/Meshes/SM_Frame5_01.SM_Frame5_01")
      (set `self.FrameNull` true))))

(fn `CleanFunction`
  (bind _paintablecanvas (`self.PaintableCanvas`))
  (`KismetRenderingLibrary.ClearRenderTarget2D` _paintablecanvas (`TextureRenderTarget2D.ClearColor` _paintablecanvas))
  (set `self.PointCheck` 0))

(fn `InitializeArt`
  (if (`self.IsArtRandomized`)
    (`self.RandomizePainting`)
    (else
      (`self.SetPainting`))))

(fn `PaintFunction`
  (returns (IsPaintable :type Boolean))
  (bind _transformcomponent (`PlayerCameraManager.TransformComponent` (`GameplayStatics.GetPlayerCameraManager` 0)))
  (bind _returnvalue (`SceneComponent.K2_GetComponentLocation` _transformcomponent))
  (bind (_hitlocation _hitnormal _bonename _outhit _returnvalue_2) (`PrimitiveComponent.K2_LineTraceComponent` (`self.PaintArea`) _returnvalue (+ _returnvalue (* (`SceneComponent.GetForwardVector` _transformcomponent) 5000.0)) true false false))
  (if _returnvalue_2
    (if (`PlayerController.IsInputKeyDown` (`GameplayStatics.GetPlayerController` 0) "LeftMouseButton")
      (`KismetSystemLibrary.DrawDebugSphere` _hitlocation 50.0 12 (struct :`R` 0.953125 :`G` 0.585783 :`B` 0.049424 :`A` 1.0) 0.0 3.0)
      (bind (_canvas _size) (`KismetRenderingLibrary.BeginDrawCanvasToRenderTarget` (`self.PaintableCanvas`)))
      (`Canvas.K2_DrawPolygon` _canvas null (* (`GameplayStatics.FindCollisionUV` _outhit 1) _size) (`self.BrushSize`) 16 (struct :`R` 1.0 :`G` 1.0 :`B` 1.0 :`A` 1.0))
      (else
        (`KismetSystemLibrary.DrawDebugSphere` _hitlocation 50.0 12 (struct :`R` 0.866667 :`G` 0.859006 :`B` 0.836025 :`A` 1.0) 0.0 3.0)
        (if (`PlayerController.IsInputKeyDown` (`GameplayStatics.GetPlayerController` 0) "RightMouseButton")
          (`KismetSystemLibrary.DrawDebugSphere` _hitlocation 50.0 12 (struct :`R` 0.18138 :`G` 1.0 :`B` 0.295803 :`A` 1.0) 0.0 3.0)
          (bind (_canvas_2 _size_2) (`KismetRenderingLibrary.BeginDrawCanvasToRenderTarget` (`self.PaintableCanvas`)))
          (`Canvas.K2_DrawPolygon` _canvas_2 null (* (`GameplayStatics.FindCollisionUV` _outhit) _size_2) (`self.BrushSize`) 16 (`TextureRenderTarget2D.ClearColor` (`self.PaintableCanvas`))))))
    (else
      (return false))))

(fn `RandomizePainting`
  (set `self.PictureFrame` (`KismetArrayLibrary.Array_Random` (`self.FrameArray`)))
  (set `self.Art` (`KismetArrayLibrary.Array_Random` (`self.ArtArray`)))
  (`self.SetPainting`))

(fn `SetPainting`
  (bind _frame (`self.Frame`))
  (bind _picture (`self.Picture`))
  (bind _frame_2 (`self.Frame`))
  (bind _pictureframe (`self.PictureFrame`))
  (bind _picture_2 (`self.Picture`))
  (bind _art (`self.Art`))
  (`self.CheckIfNullPainting`)
  (if (`self.FrameNull`)
    (`StaticMeshComponent.SetStaticMesh` _frame (`self.PictureFrame`))
    (`PrimitiveComponent.SetMaterial` _frame 0 "/Game/StarterContent/LevelPrototyping/Materials/MI_PrototypeGrid_Gray_02.MI_PrototypeGrid_Gray_02")
    (else
      (`StaticMeshComponent.SetStaticMesh` _frame_2 _pictureframe)
      (`PrimitiveComponent.SetMaterial` _frame_2 0 (`StaticMesh.GetMaterial` _pictureframe 0))))
  (if (`self.ArtNull`)
    (`StaticMeshComponent.SetStaticMesh` _picture (`self.Art`))
    (`PrimitiveComponent.SetMaterial` _picture 0 "/Engine/EditorMeshes/Camera/MI_RailRig.MI_RailRig")
    (else
      (`StaticMeshComponent.SetStaticMesh` _picture_2 _art)
      (`PrimitiveComponent.SetMaterial` _picture_2 0 (`StaticMesh.GetMaterial` _art 0)))))

(fn `UserConstructionScript`)