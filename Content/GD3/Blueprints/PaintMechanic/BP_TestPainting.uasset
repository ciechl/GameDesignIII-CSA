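; Test Blueprint for painting on a cube by aiming the camera and holding the left mouse button.
; BeginPlay clears the PaintableCanvas render target, then Tick line-traces the Cube component along the camera's forward vector.
; On a hit, a debug sphere shows the aim point, and holding the button draws a small polygon at the collision UV on the canvas.
; The draw has no matching EndDrawCanvasToRenderTarget call.
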(event `self.ReceiveBeginPlay`
  (bind _paintablecanvas (`self.PaintableCanvas`))
  (`KismetRenderingLibrary.ClearRenderTarget2D` _paintablecanvas (`TextureRenderTarget2D.ClearColor` _paintablecanvas)))

(event `self.ReceiveTick`
  (params (DeltaSeconds :type "Float (single-precision)"))
  (bind _transformcomponent (`PlayerCameraManager.TransformComponent` (`GameplayStatics.GetPlayerCameraManager` 0)))
  (bind _returnvalue (`SceneComponent.K2_GetComponentLocation` _transformcomponent))
  (bind (_hitlocation _hitnormal _bonename _outhit _returnvalue_2) (`PrimitiveComponent.K2_LineTraceComponent` (`self.Cube`) _returnvalue (+ _returnvalue (* (`SceneComponent.GetForwardVector` _transformcomponent) 5000.0)) true false false))
  (if _returnvalue_2
    (if (`PlayerController.IsInputKeyDown` (`GameplayStatics.GetPlayerController` 0) "LeftMouseButton")
      (`KismetSystemLibrary.DrawDebugSphere` _hitlocation 50.0 12 (struct :`R` 0.953125 :`G` 0.585783 :`B` 0.049424 :`A` 1.0) 0.0 3.0)
      (bind (_canvas _size) (`KismetRenderingLibrary.BeginDrawCanvasToRenderTarget` (`self.PaintableCanvas`)))
      (`Canvas.K2_DrawPolygon` _canvas null (* (`GameplayStatics.FindCollisionUV` _outhit) _size) (1.0 1.0) 16 (struct :`R` 1.0 :`G` 1.0 :`B` 1.0 :`A` 1.0))
      (else
        (`KismetSystemLibrary.DrawDebugSphere` _hitlocation 50.0 12 (struct :`R` 0.041667 :`G` 0.037741 :`B` 0.034288 :`A` 1.0) 0.0 3.0)))))

(fn `UserConstructionScript`)