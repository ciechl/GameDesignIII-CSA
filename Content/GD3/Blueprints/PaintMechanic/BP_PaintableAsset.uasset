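; BP_PaintableAsset is a paintable object Blueprint that holds its own render-target canvas for team-colored paint.
; On BeginPlay it creates and clears the canvas, then creates a dynamic instance of M_PaintMat without assigning it or binding the canvas.
; DrawFunction turns the stored hit into a collision UV and draws a brush-sized polygon there in TeamColor.
; Its only call here is unwired, and it never ends the canvas draw.
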(event `self.ReceiveBeginPlay`
  (bind _returnvalue (`KismetRenderingLibrary.CreateRenderTarget2D` 512 512 "RTF_RGBA8"))
  (bind _output_get (set `self.PaintableCanvas` _returnvalue))
  (`KismetRenderingLibrary.ClearRenderTarget2D` _output_get (`TextureRenderTarget2D.ClearColor` _output_get))
  (`KismetMaterialLibrary.CreateDynamicMaterialInstance` "/Game/GD3/Blueprints/PaintMechanic/BaseMechanic/M_PaintMat.M_PaintMat"))

(fn `DrawFunction`
  (bind (_canvas _size) (`KismetRenderingLibrary.BeginDrawCanvasToRenderTarget` (`self.PaintableCanvas`)))
  (`Canvas.K2_DrawPolygon` _canvas null (* (`GameplayStatics.FindCollisionUV` (`self.UVHitLocation`)) _size) (`self.BrushSize`) 16 (`self.TeamColor`)))

(fn `UserConstructionScript`)