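; Projectile that leaves paint-style decals where it hits and shoves physics objects.
; On Hit it applies a velocity-scaled impulse to simulating components, then attaches a random decal material at a randomized size, oriented to the surface normal.
; DoOnce gates limit decal spawning: actors tagged Paintable get only the decal, while other hits also destroy the projectile.
; The Player tag check has no effect.
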(event `self.ReceiveHit`
  (params (MyComp :type "PrimitiveComponent Object Reference") (Other :type "Actor Object Reference") (OtherComp :type "PrimitiveComponent Object Reference") (bSelfMoved :type Boolean) (HitLocation :type "Vector Structure") (HitNormal :type "Vector Structure") (NormalImpulse :type "Vector Structure") (Hit :type "HitResult Structure (by ref)"))
  (bind _returnvalue (`KismetMathLibrary.Conv_VectorToRotator` HitNormal))
  (`|ExecutionSequence`
    (:`then_0`
      (if (`SceneComponent.IsSimulatingPhysics` OtherComp "None")
        (`PrimitiveComponent.AddImpulseAtLocation` OtherComp (* (`self.GetVelocity`) (`KismetMathLibrary.Conv_DoubleToVector` 100.0)) (`self.K2_GetActorLocation`) "None")))
    (:`then_1`
      (bind _output_get (set `self.RandomSize` (`KismetMathLibrary.RandomFloatInRange` 0.0 75.0)))
      (if (`self.ActorHasTag` Other "Paintable")
        (`/Engine/EditorBlueprintResources/StandardMacros.DoOnce` false
          (:`Completed`
            (bind _returnvalue_2 (+ _output_get (`self.DefaultY`)))
            (bind _returnvalue_3 (+ _output_get (`self.DefaultZ`)))
            (`GameplayStatics.SpawnDecalAttached` (`KismetArrayLibrary.Array_Random` (`self.Decal Material`)) (`KismetMathLibrary.MakeVector` 28.0 _returnvalue_2 _returnvalue_3) OtherComp "None" HitLocation _returnvalue "KeepWorldPosition")))
        (else
          (if (`self.ActorHasTag` Other "Player")
            _
            (else
              _))
          (`/Engine/EditorBlueprintResources/StandardMacros.DoOnce` false
            (:`Completed`
              (`GameplayStatics.SpawnDecalAttached` (`KismetArrayLibrary.Array_Random` (`self.Decal Material`)) (`KismetMathLibrary.MakeVector` 28.0 _returnvalue_2 _returnvalue_3) OtherComp "None" HitLocation _returnvalue "KeepWorldPosition")
              (if (not (`self.WasDestroyed`))
                (set `self.WasDestroyed` true)
                (`/Engine/EditorBlueprintResources/StandardMacros.DoOnce` false
                  (:`Completed`
                    (`self.K2_DestroyActor`)))))))))))

(fn `UserConstructionScript`)